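; BP_PlayerController is the player controller that turns mouse and keyboard input into game actions.
; On BeginPlay it finds and caches the BP_GameSystem actor.
; A left click traces under the cursor and, if it hits an unmarked BP_Cell, passes that cell to the game system's MakeTurn.
; Escape and a debug Tab key both call the game system's CallOnGamePause.
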(event EventBeginPlay
  (bind _returnvalue (Actor|GetActorOfClass "/Game/Objects/Systems/BP_GameSystem.BP_GameSystem_C"))
  (Variables|Default|SetGameSystem _returnvalue))

(event Input|KeyboardEvents|DebugKeyTab
  (params (Key :type Key%20Structure :default "None") (ActionValue :type Input%20Action%20Value%20Structure))
  (:Pressed
    (Default|CallOnGamePause (Variables|Default|GetGameSystem))))

(event Input|MouseEvents|LeftMouseButton
  (params (Key :type Key%20Structure :default "None"))
  (:Pressed
    (bind _asbp_cell (Utilities|Casting|CastToBP_Cell (.HitActor (Collision|BreakHitResult (.HitResult (Game|Player|GetHitResultUnderCursorbyChannel self "TraceTypeQuery1" true))))))
    (if (not (Variables|/Game/Objects/BP_Cell.BP_Cell_C|GetIsCellMarked _asbp_cell))
      (Class|GameSystem|MakeTurn (Variables|Default|GetGameSystem) _asbp_cell))))

(event Input|KeyboardEvents|Escape
  (params (Key :type Key%20Structure :default "None"))
  (:Pressed
    (Default|CallOnGamePause (Variables|Default|GetGameSystem))))

(fn ConstructionScript)