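; BP_Cell is a board cell actor that holds a single mark, shown as a static mesh.
; On BeginPlay it caches the BP_GameSystem and BP_AudioSystem actors found in the level.
; AddMark creates a mesh component at runtime from the passed mesh, flags the cell as marked and plays the mark sound.
; ClearCell calls RemoveMark to destroy that component, then resets MarkBool.
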(event `self.ReceiveBeginPlay`
  (bind _returnvalue (`GameplayStatics.GetActorOfClass` "/Game/Objects/Systems/BP_GameSystem.BP_GameSystem_C"))
  (set `self.GameSystem` _returnvalue)
  (bind _returnvalue_2 (`GameplayStatics.GetActorOfClass` "/Game/Objects/Systems/BP_AudioSystem.BP_AudioSystem_C"))
  (set `self.AudioSystem` _returnvalue_2))

(event `AddMark`
  (params (NewParam :type "StaticMesh Object Reference"))
  (`KismetSystemLibrary.PrintText` (`|FormatText` "Cell '{index}' set mark '{mark}'" (`KismetSystemLibrary.GetDisplayName` self) (`KismetSystemLibrary.GetDisplayName` NewParam)))
  (bind _returnvalue (`AddComponent|NODE_AddStaticMeshComponent-0`))
  (bind _output_get (set `self.Mark` _returnvalue))
  (`StaticMeshComponent.SetStaticMesh` _output_get NewParam)
  (set `self.IsCellMarked` true)
  (`/Game/Objects/Systems/BP_AudioSystem.PlayMark` (`self.AudioSystem`)))

(event `RemoveMark`
  (bind _mark (`self.Mark`))
  (if (`KismetSystemLibrary.IsValid` _mark)
    (`ActorComponent.K2_DestroyComponent` _mark)
    (set `self.IsCellMarked` false)))

(fn `ClearCell`
  (`self.RemoveMark`)
  (set `self.MarkBool` false))

(fn `UserConstructionScript`)