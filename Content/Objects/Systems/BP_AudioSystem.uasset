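; Audio system Blueprint for an X-and-O mark game, exposing events for music and sound effects.
; PlayMusic creates a lowered-pitch 2D sound and fades it in to MusicVolume, while PlayMark plays a one-shot mark cue.
; StopWin stops a valid, active WinSound.
; PlayWin is empty: the logic that creates WinSound and sets its Winner parameter is disconnected, so it never runs.
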(event `self.PlayMusic`
  (params (Sound :type "SoundBase Object Reference"))
  (bind _returnvalue (`GameplayStatics.CreateSound2D` Sound 1.0 0.75 0.0 null))
  (bind _output_get (set `self.Music` _returnvalue))
  (`AudioComponent.FadeIn` _output_get 5.0 (`self.Music_Volume`) 0.0 "Linear"))

(event `self.PlayWin`
  (params (Winner :type "EMark Enum" :default "None")))

(event `self.StopWin`
  (bind _winsound (`self.WinSound`))
  (`/Engine/EditorBlueprintResources/StandardMacros.IsValid` _winsound
    (:`Is Valid`
      (switch `EAudioComponentPlayState` (`AudioComponent.GetPlayState` _winsound)
        (:`Playing`
          _)
        (:`Paused`
          _)
        (:`FadingIn`
          _)
        (:`FadingOut`
          _))
      (`AudioComponent.Stop` (`self.WinSound`)))))

(event `self.PlayMark`
  (`GameplayStatics.PlaySound2D` "/Game/Resources/Audio/SFX/SC_Mark.SC_Mark" 1.0 1.0 0.0 null null))

(fn `UserConstructionScript`)