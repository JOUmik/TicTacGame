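; Game manager for an X/O m,n,k board game (generalized tic-tac-toe), handling turns, win and draw detection, and restarts.
; PrepareGame creates the UI and spawns an M×N cell grid with divider lines, stored in a flat array.
; MakeTurn marks cells and scans from the latest move, using FlipFlop to total opposite directions toward K in a row.
; It recolors the light per turn, highlights winning cells and plays end-game audio.
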(event `PrepareGame`
  (`|ExecutionSequence`
    (:`then_0`
      (bind _returnvalue (`|CreateWidget` "/Game/Widgets/WBP_GameUI.WBP_GameUI_C"))
      (`UserWidget.AddToViewport` _returnvalue 0)
      (`self.onGameStart`)
      (`self.onTurnChange`))
    (:`then_1`
      (`self.SetupCells`))
    (:`then_3`
      (`self.HandleBackgroundColor`))
    (:`then_4`
      (bind _returnvalue_2 (`GameplayStatics.GetActorOfClass` "/Game/Objects/Systems/BP_AudioSystem.BP_AudioSystem_C"))
      (set `self.AudioSystem` _returnvalue_2))))

(fn `CalcLineTransform`
  (params (Cell :type "/Game/Objects/BP_Cell Object Reference") (Line_Info :type "Map of String to Boolean"))
  (returns (Line_Transform :type "Transform Structure"))
  (bind (_origin _boxextent) (`self.GetActorBounds` Cell false false))
  (bind _returnvalue (`self.GetTransform` Cell))
  (bind _cellsoffsetperc (`self.CellsOffsetPerc`))
  (bind _cellsoffsetperc_2 (`self.CellsOffsetPerc`))
  (bind _returnvalue_2 (* (/ (.x (.scale _returnvalue)) 100.0) _cellsoffsetperc))
  (bind _returnvalue_3 (* (/ (.y (.scale _returnvalue)) 100.0) (+ 100.0 _cellsoffsetperc)))
  (bind _returnvalue_4 (* (/ (.z (.scale _returnvalue)) 100.0) _cellsoffsetperc))
  (if (`BlueprintMapLibrary.Map_Find` Line_Info "Left")
    (return (`KismetMathLibrary.MakeTransform` (`KismetMathLibrary.MakeVector` (.x (.location _returnvalue)) (- (.y (.location _returnvalue)) (.y _boxextent) (* (/ (.y _boxextent) 100.0) _cellsoffsetperc_2)) (.z (.location _returnvalue))) (`KismetMathLibrary.MakeRotator` (.roll (.rotation _returnvalue)) (.pitch (.rotation _returnvalue)) (+ (.yaw (.rotation _returnvalue)) 90.0)) (`KismetMathLibrary.MakeVector` _returnvalue_2 _returnvalue_3 _returnvalue_4)))
    (elif (`BlueprintMapLibrary.Map_Find` Line_Info "Top")
      (return (`KismetMathLibrary.MakeTransform` (`KismetMathLibrary.MakeVector` (- (.x (.location _returnvalue)) (.x _boxextent) (* (/ (.x _boxextent) 100.0) _cellsoffsetperc_2)) (.y (.location _returnvalue)) (.z (.location _returnvalue))) (`KismetMathLibrary.MakeRotator` (.roll (.rotation _returnvalue)) (.pitch (.rotation _returnvalue)) (.yaw (.rotation _returnvalue))) (`KismetMathLibrary.MakeVector` _returnvalue_2 _returnvalue_3 _returnvalue_4))))))

(fn `ChangeWinCellsColor`
  (locals (LineType :type String))
  (for _array_element (`self.Cells`)
    (if (`/Game/Objects/BP_Cell.IsCellMarked` _array_element)
      (if (`KismetArrayLibrary.Array_Contains` (`self.WinCells`) _array_element)
        (bind _mark (`/Game/Objects/BP_Cell.Mark` _array_element))
        (`PrimitiveComponent.SetMaterial` _mark 0 "/Game/Resources/Materials/MI_Green.MI_Green")
        (else
          (`PrimitiveComponent.SetMaterial` _mark 0 "/Game/Resources/Materials/M_Basic.M_Basic"))))))

(fn `CheckClickedCellSiblingsForWin`
  (locals (MarkCounter :type Integer) (Direction :type "/Game/Resources/Enums/E_Directions Enum") (DirectionCheck :type Boolean) (DirectionCellX :type Integer) (DirectionCellY :type Integer) (DirectionCellIndex :type Integer))
  (bind _directioncellindex (`local.DirectionCellIndex`))
  (bind _directioncellindex_2 (`local.DirectionCellIndex`))
  (bind _directioncellindex_3 (`local.DirectionCellIndex`))
  (bind _clickedcell (`self.ClickedCell`))
  (bind _directioncellindex_4 (`local.DirectionCellIndex`))
  (bind _clickedcell_2 (`self.ClickedCell`))
  (bind _clickedcell_3 (`self.ClickedCell`))
  (bind _wincells (`self.WinCells`))
  (bind _clickedcell_4 (`self.ClickedCell`))
  (bind _clickedcell_5 (`self.ClickedCell`))
  (bind _clickedcell_6 (`self.ClickedCell`))
  (bind _clickedcell_7 (`self.ClickedCell`))
  (bind _clickedcell_8 (`self.ClickedCell`))
  (bind _returnvalue (- (`/Game/Objects/BP_Cell.Y` _clickedcell_4) (`local.DirectionCellIndex`)))
  (bind _returnvalue_2 (+ (`/Game/Objects/BP_Cell.Y` _clickedcell_5) (`local.DirectionCellIndex`)))
  (bind _returnvalue_3 (+ (`/Game/Objects/BP_Cell.Y` _clickedcell) _directioncellindex))
  (bind _returnvalue_4 (- (`/Game/Objects/BP_Cell.X` _clickedcell) _directioncellindex))
  (bind _returnvalue_5 (- (`/Game/Objects/BP_Cell.X` _clickedcell_2) (`local.DirectionCellIndex`)))
  (bind _returnvalue_6 (+ (`/Game/Objects/BP_Cell.X` _clickedcell_3) (`local.DirectionCellIndex`)))
  (bind _returnvalue_7 (+ (`/Game/Objects/BP_Cell.X` _clickedcell_8) _directioncellindex_4))
  (bind _returnvalue_8 (- (`/Game/Objects/BP_Cell.X` _clickedcell_6) _directioncellindex_2))
  (bind _returnvalue_9 (- (`/Game/Objects/BP_Cell.Y` _clickedcell_6) _directioncellindex_2))
  (bind _returnvalue_10 (+ (`/Game/Objects/BP_Cell.X` _clickedcell_7) _directioncellindex_3))
  (bind _returnvalue_11 (+ (`/Game/Objects/BP_Cell.Y` _clickedcell_7) _directioncellindex_3))
  (bind _returnvalue_12 (- (`/Game/Objects/BP_Cell.Y` _clickedcell_8) _directioncellindex_4))
  (for _index (range (enumcount `/Game/Resources/Enums/E_Directions`)) :!label _label
    (bind _output_get (set `local.Direction` (cast `/Game/Resources/Enums/E_Directions` (`KismetMathLibrary.Conv_IntToByte` _index))))
    (switch `/Game/Resources/Enums/E_Directions` _output_get
      (:`NewEnumerator0`
        _)
      (:`NewEnumerator1`
        _)
      (:`NewEnumerator2`
        _)
      (:`NewEnumerator3`
        _)
      (:`NewEnumerator4`
        _)
      (:`NewEnumerator5`
        _)
      (:`NewEnumerator6`
        _)
      (:`NewEnumerator7`
        _))
    (`/Engine/EditorBlueprintResources/StandardMacros.FlipFlop`
      (:`A`
        (`KismetArrayLibrary.Array_Clear` _wincells)
        (`KismetArrayLibrary.Array_Add` _wincells (`self.ClickedCell`))
        (set `local.MarkCounter` 0))
      (:`B`
        _))
    (for _index_2 (range 1 (`self.K`))
      (set `local.DirectionCellIndex` _index_2)
      (switch `/Game/Resources/Enums/E_Directions` (`local.Direction`)
        (:`NewEnumerator0`
          (set `local.DirectionCheck` (>= _returnvalue_5 1))
          (set `local.DirectionCellX` _returnvalue_5)
          (set `local.DirectionCellY` (`/Game/Objects/BP_Cell.Y` _clickedcell_2)))
        (:`NewEnumerator1`
          (set `local.DirectionCheck` (<= _returnvalue_6 (`self.M`)))
          (set `local.DirectionCellX` _returnvalue_6)
          (set `local.DirectionCellY` (`/Game/Objects/BP_Cell.Y` _clickedcell_3)))
        (:`NewEnumerator2`
          (set `local.DirectionCheck` (>= _returnvalue 1))
          (set `local.DirectionCellX` (`/Game/Objects/BP_Cell.X` _clickedcell_4))
          (set `local.DirectionCellY` _returnvalue))
        (:`NewEnumerator3`
          (set `local.DirectionCheck` (<= _returnvalue_2 (`self.N`)))
          (set `local.DirectionCellX` (`/Game/Objects/BP_Cell.X` _clickedcell_5))
          (set `local.DirectionCellY` _returnvalue_2))
        (:`NewEnumerator4`
          (set `local.DirectionCheck` (and (>= _returnvalue_8 1) (>= _returnvalue_9 1)))
          (set `local.DirectionCellX` _returnvalue_8)
          (set `local.DirectionCellY` _returnvalue_9))
        (:`NewEnumerator5`
          (set `local.DirectionCheck` (and (<= _returnvalue_10 (`self.M`)) (<= _returnvalue_11 (`self.N`))))
          (set `local.DirectionCellX` _returnvalue_10)
          (set `local.DirectionCellY` _returnvalue_11))
        (:`NewEnumerator6`
          (set `local.DirectionCheck` (and (<= _returnvalue_7 (`self.M`)) (>= _returnvalue_12 1)))
          (set `local.DirectionCellX` _returnvalue_7)
          (set `local.DirectionCellY` _returnvalue_12))
        (:`NewEnumerator7`
          (set `local.DirectionCheck` (and (>= _returnvalue_4 1) (<= _returnvalue_3 (`self.N`))))
          (set `local.DirectionCellX` _returnvalue_4)
          (set `local.DirectionCellY` _returnvalue_3)))
      (if (`local.DirectionCheck`)
        (bind _result (`self.GetCellByIndex` (`local.DirectionCellX`) (`local.DirectionCellY`)))
        (if (`/Game/Objects/BP_Cell.IsCellMarked` _result)
          (if (== (`/Game/Objects/BP_Cell.MarkBool` _result) (`/Game/Objects/BP_Cell.MarkBool` (`self.ClickedCell`)))
            (`KismetArrayLibrary.Array_Add` (`self.WinCells`) _result)
            (bind _result_2 (`/Engine/EditorBlueprintResources/StandardMacros.IncrementInt` (`local.MarkCounter`))
              (:`  `
                (if (== _result_2 (- (`self.K`) 1))
                  (set `self.IsGameEnd` true)
                  (`|ExecutionSequence`
                    (:`then_0`
                      (break))
                    (:`then_1`
                      (goto _label :!via `Break`))
                    (:`then_2`
                      (if (`/Game/Objects/BP_Cell.MarkBool` (`self.ClickedCell`))
                        (set `self.Winner` "X")
                        (else
                          (set `self.Winner` "O"))))))))
            (else
              (break)))
          (else
            (break)))
        (else
          (break))))))

(fn `ClearAllCells`
  (for _array_element (`self.Cells`)
    (`/Game/Objects/BP_Cell.ClearCell` _array_element)))

(fn `GetCellByIndex`
  (params (X :type Integer) (Y :type Integer))
  (returns (Result :type "/Game/Objects/BP_Cell Object Reference"))
  (return (`|GetArrayItem` (`self.Cells`) (- (+ (* (- X 1) (`self.N`)) Y) 1))))

(fn `HandleBackgroundColor`
  (bind _returnvalue (`GameplayStatics.GetActorOfClass` "/Script/Engine.DirectionalLight"))
  (if (not (`self.IsGameEnd`))
    (if (`self.Turn`)
      (bind _lightcomponent (`Light.LightComponent` _returnvalue))
      (`LightComponent.SetLightColor` _lightcomponent (struct :`R` 1.0 :`B` 0.112386 :`A` 1.0) true)
      (else
        (`LightComponent.SetLightColor` _lightcomponent (struct :`R` 0.333333 :`B` 1.0 :`A` 1.0) true)))))

(fn `MakeTurn`
  (params (ClickedCell :type "/Game/Objects/BP_Cell Object Reference"))
  (bind _clickedcell (`self.ClickedCell`))
  (bind _clickedcell_2 (`self.ClickedCell`))
  (set `self.ClickedCell` ClickedCell)
  (if (not (`self.IsGameEnd`))
    (if (`self.Turn`)
      (`/Game/Objects/BP_Cell.AddMark` _clickedcell_2 "/Game/Resources/Meshes/X.X")
      (set `/Game/Objects/BP_Cell.MarkBool` true _clickedcell)
      (else
        (`/Game/Objects/BP_Cell.AddMark` _clickedcell_2 "/Game/Resources/Meshes/O.O")
        (set `/Game/Objects/BP_Cell.MarkBool` false _clickedcell)))
    (set `self.Turn` (not (`self.Turn`)))
    (`/Engine/EditorBlueprintResources/StandardMacros.DecrementInt` (`self.AvailableMoves`)
      (:`  `
        (`self.CheckClickedCellSiblingsForWin`)
        (`self.HandleBackgroundColor`)
        (`self.onTurnChange`)
        (if (`self.IsGameEnd`)
          (switch `EMark` (`self.Winner`)
            (:`X`
              (`/Engine/EditorBlueprintResources/StandardMacros.IncrementInt` (`self.WinCountX`)
                (:`  `
                  _)))
            (:`O`
              (`/Engine/EditorBlueprintResources/StandardMacros.IncrementInt` (`self.WinCountO`)
                (:`  `
                  _))))
          (`self.ChangeWinCellsColor`)
          (`/Game/Objects/Systems/BP_AudioSystem.PlayWin` (`self.AudioSystem`) (`self.Winner`) :!label _label)
          (`self.onGameEnd`)
          (elif (< (`self.AvailableMoves`) 1)
            (set `self.IsGameEnd` true)
            (`self.onTurnChange`)
            (goto _label)))))))

(fn `ResetGameData`
  (set `self.IsGameEnd` false)
  (set `self.Winner` "None")
  (set `self.Turn` true)
  (`self.onTurnChange`)
  (set `self.AvailableMoves` (`KismetArrayLibrary.Array_Length` (`self.Cells`)))
  (`self.HandleBackgroundColor`))

(fn `RestartGame`
  (`self.ClearAllCells`)
  (`self.ResetGameData`)
  (`/Game/Objects/Systems/BP_AudioSystem.StopWin` (`self.AudioSystem`)))

(fn `SetCellByIndex`
  (params (Cell :type "/Game/Objects/BP_Cell Object Reference"))
  (`KismetArrayLibrary.Array_Set` (`self.Cells`) (- (+ (* (- (`/Game/Objects/BP_Cell.X` Cell) 1) (`self.N`)) (`/Game/Objects/BP_Cell.Y` Cell)) 1) Cell true))

(fn `SetCellLines`
  (params (Cell :type "/Game/Objects/BP_Cell Object Reference"))
  (`|ExecutionSequence`
    (:`then_0`
      (if (> (`/Game/Objects/BP_Cell.X` Cell) 1)
        (bind _line_transform (`self.CalcLineTransform` Cell (`|MakeMap` "Left" true)))
        (`|SpawnActorFromClass` "/Game/Objects/BP_Line.BP_Line_C" _line_transform "Undefined" "MultiplyWithRoot" null null)))
    (:`then_1`
      (if (> (`/Game/Objects/BP_Cell.Y` Cell) 1)
        (bind _line_transform_2 (`self.CalcLineTransform` Cell (`|MakeMap` "Top" true)))
        (`|SpawnActorFromClass` "/Game/Objects/BP_Line.BP_Line_C" _line_transform_2 "Undefined" "MultiplyWithRoot" null null)))))

(fn `SetCellTransform`
  (params (Cell :type "/Game/Objects/BP_Cell Object Reference"))
  (bind (_origin _boxextent) (`self.GetActorBounds` Cell false false))
  (bind _x (`/Game/Objects/BP_Cell.X` Cell))
  (bind _y (`/Game/Objects/BP_Cell.Y` Cell))
  (bind _cellsoffsetperc (`self.CellsOffsetPerc`))
  (bind _returnvalue (* (.x _boxextent) 2.0))
  (bind _returnvalue_2 (* (.y _boxextent) 2.0))
  (bind _returnvalue_3 (* (/ (.x _boxextent) 100.0) _cellsoffsetperc 2.0))
  (bind _returnvalue_4 (* (/ (.y _boxextent) 100.0) _cellsoffsetperc 2.0))
  (`self.K2_SetActorTransform` Cell (`KismetMathLibrary.MakeTransform` (`KismetMathLibrary.MakeVector` (- (+ (- (* _returnvalue _y) _returnvalue) (* _returnvalue_3 _y)) _returnvalue_3) (- (+ (- (* _returnvalue_2 _x) _returnvalue_2) (* _returnvalue_4 _x)) _returnvalue_4))) false false))

(fn `SetupCells`
  (for _index (range 1 (+ (`self.M`) 1))
    (for _index_2 (range 1 (+ (`self.N`) 1))
      (bind _returnvalue (`|SpawnActorFromClass` "/Game/Objects/BP_Cell.BP_Cell_C" (`KismetMathLibrary.MakeTransform` (0.0 0.0 0.0)) "Undefined" "MultiplyWithRoot" null 0 0 null))
      (set `/Game/Objects/BP_Cell.Y` _index_2 _returnvalue)
      (set `/Game/Objects/BP_Cell.X` _index _returnvalue)
      (`self.SetCellByIndex` _returnvalue)
      (`self.SetCellTransform` _returnvalue)
      (`self.SetCellLines` _returnvalue)))
  (set `self.AvailableMoves` (`KismetArrayLibrary.Array_Length` (`self.Cells`))))

(fn `UserConstructionScript`)